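; BP_BaseballBat is a melee weapon actor for a baseball bat that knocks physics objects around and triggers Chaos physics fields on impact.
; On Hit, it applies an impulse scaled from its velocity to any simulating component, at the bat's location.
; Every hit also spawns a scaled-down, short-lived FS_MasterField slightly behind the struck surface, sets its radial magnitude and triggers it.
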(event `self.ReceiveHit`
  (params (MyComp :type "PrimitiveComponent Object Reference") (Other :type "Actor Object Reference") (OtherComp :type "PrimitiveComponent Object Reference") (bSelfMoved :type Boolean) (HitLocation :type "Vector Structure") (HitNormal :type "Vector Structure") (NormalImpulse :type "Vector Structure") (Hit :type "HitResult Structure (by ref)"))
  (bind (_bblockinghit _binitialoverlap _time _distance _location _impactpoint _normal _impactnormal) (`GameplayStatics.BreakHitResult` Hit))
  (bind (_returnvalue_location _returnvalue_rotation) (`KismetMathLibrary.BreakTransform` (`KismetMathLibrary.Conv_VectorToTransform` _impactpoint)))
  (if (`SceneComponent.IsSimulatingPhysics` OtherComp "None")
    (`PrimitiveComponent.AddImpulseAtLocation` OtherComp (* (`self.GetVelocity`) (100.0 100.0 100.0)) (`self.K2_GetActorLocation`) "None"))
  (bind _returnvalue (`|SpawnActorFromClass` "/Engine/EditorResources/FieldNodes/FS_MasterField.FS_MasterField_C" (`KismetMathLibrary.MakeTransform` (+ _returnvalue_location (* _impactnormal (-3.0 -3.0 -3.0))) _returnvalue_rotation (0.7 0.7 0.7)) "Undefined" "MultiplyWithRoot" null null))
  (set `self.ChaosImpactChaosField` _returnvalue)
  (set `/Engine/EditorResources/FieldNodes/FS_MasterField.ActivationType` "NewEnumerator4" (`self.ChaosImpactChaosField`))
  (`self.SetLifeSpan` (`self.ChaosImpactChaosField`) 0.1)
  (set `/Engine/EditorResources/FieldNodes/FS_MasterField.Radial Magnitude` 150.0 (`self.ChaosImpactChaosField`))
  (`/Engine/EditorResources/FieldNodes/FS_MasterField.CE_Trigger` (`self.ChaosImpactChaosField`)))

(fn `UserConstructionScript`)